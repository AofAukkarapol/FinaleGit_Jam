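; BP_testRight is a moving hazard actor that damages the player on contact.
; On BeginPlay the Move timeline drives the skeletal mesh's relative location, and a Delay on its update pin destroys the actor about five seconds later.
; When a Player-tagged actor overlaps the Box, it spawns an explosion at the mesh, subtracts one HP from BP_ThirdPersonCharacter, prints the result and destroys itself.
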(event `self.ReceiveBeginPlay`
  (bind (_direction _newtrack_0) (`Timeline|Move`)
    (:`Update`
      (`SceneComponent.K2_SetRelativeLocation` (`self.SkeletalMesh`) _newtrack_0 false false)
      (`KismetSystemLibrary.Delay` 5.0)
      (`self.K2_DestroyActor`))))

(event `self.Box.OnComponentBeginOverlap`
  (params (OverlappedComponent :type "PrimitiveComponent Object Reference") (OtherActor :type "Actor Object Reference") (OtherComp :type "PrimitiveComponent Object Reference") (OtherBodyIndex :type Integer) (bFromSweep :type Boolean) (SweepResult :type "HitResult Structure (by ref)"))
  (if (`self.ActorHasTag` OtherActor "Player")
    (`GameplayStatics.SpawnEmitterAtLocation` "/Game/StarterContent/Particles/P_Explosion.P_Explosion" (`SceneComponent.K2_GetComponentLocation` (`self.SkeletalMesh`)))
    (bind _asbp_third_person_character (cast `/Game/ThirdPerson/Blueprints/BP_ThirdPersonCharacter` OtherActor))
    (bind _output_get (set `/Game/ThirdPerson/Blueprints/BP_ThirdPersonCharacter.HP` (- (`/Game/ThirdPerson/Blueprints/BP_ThirdPersonCharacter.HP` _asbp_third_person_character) 1) _asbp_third_person_character))
    (`KismetSystemLibrary.PrintString` (`KismetStringLibrary.Conv_IntToString` _output_get))
    (`self.K2_DestroyActor`)))

(fn `UserConstructionScript`)